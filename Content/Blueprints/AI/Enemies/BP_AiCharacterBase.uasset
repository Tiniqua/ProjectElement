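; BP_AiCharacterBase is an AI enemy character Blueprint that displays a health bar through its HealthWidget component.
; On BeginPlay it creates a WBP_EnemyHealthBar, seeds its Health from the HealthVitality max amount and assigns it to the widget component.
; A handler bound to HealthVitality's received-damage event subtracts incoming damage from the bar's own Health value rather than reading it back from the vitality.
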(event `self.ReceiveBeginPlay`
  (bind _returnvalue (`|CreateWidget` "/Game/UI/HealthBar/WBP_EnemyHealthBar.WBP_EnemyHealthBar_C"))
  (bind _output_get (set `self.Instance` _returnvalue))
  (set `/Game/UI/HealthBar/WBP_EnemyHealthBar.Health` (`VitalityComponent.MaxAmount` (`self.HealthVitality`)) _output_get)
  (`WidgetComponent.SetWidget` (`self.HealthWidget`) _output_get)
  (add `VitalityComponent.OnReceivedDamageEvent` (`self.HealthVitality`) (delegate `OnReceivedDamageEvent_Event`)))

(event `OnReceivedDamageEvent_Event`
  (params (InDamage :type "Float (single-precision)") (InDamageSource :type "Actor Object Reference"))
  (bind _instance (`self.Instance`))
  (set `/Game/UI/HealthBar/WBP_EnemyHealthBar.Health` (- (`/Game/UI/HealthBar/WBP_EnemyHealthBar.Health` _instance) InDamage) _instance))

(fn `UserConstructionScript`)